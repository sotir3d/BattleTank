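; Player-controllable tank pawn Blueprint that drives, aims and fires, with a health bar widget linked back to the tank.
; BeginPlay wires barrel, turret and tracks into the TankAiming and TankMovement components, which receive fire and movement input.
; Input also rotates the gimbal and spring-arm camera, toggles first/third-person views, and plays shot audio based on firing status.
; Tick clamps roll and pitch to limit tipping; per-track throttle inputs are disconnected.
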(event `self.ReceiveBeginPlay`
  (`TankAimingComponent.Initialize` (`self.TankAiming`) (`self.Barrel`) (`self.Turret`))
  (`TankMovementComponent.Initialize` (`self.TankMovement`) (`self.LeftTrack`) (`self.RightTrack`))
  (`self.Initialize HealthBarWidget`))

(event `self.ReceiveTick`
  (params (DeltaSeconds :type "Float (single-precision)"))
  ;[1 1 1] Fix Rotation
  (`SceneComponent.K2_SetWorldRotation` (`self.Tank`) (`KismetMathLibrary.MakeRotator` (`KismetMathLibrary.ClampAngle` (.roll (`SceneComponent.K2_GetComponentRotation` (`self.Tank`))) -30.0 30.0) (`KismetMathLibrary.ClampAngle` (.pitch (`SceneComponent.K2_GetComponentRotation` (`self.Tank`))) -30.0 30.0) (.yaw (`SceneComponent.K2_GetComponentRotation` (`self.Tank`)))) false false))

(event `InputAxis|AimAzimuth`
  (params (AxisValue :type "Float (single-precision)"))
  ;[1 1 1] CameraControl
  (`SceneComponent.K2_AddLocalRotation` (`self.AzimuthGimbal`) (`KismetMathLibrary.MakeRotator` 0.0 0.0 AxisValue) false false))

(event `InputAxis|LeftTrackThrottle`
  (params (AxisValue :type "Float (single-precision)"))
  ;[1 1 1] Movement
)

(event `InputAxis|RightTrackThrottle`
  (params (AxisValue :type "Float (single-precision)"))
  ;[1 1 1] Movement
)

(event `InputAxis|AimElevation`
  (params (AxisValue :type "Float (single-precision)"))
  ;[1 1 1] CameraControl
  (`SceneComponent.K2_AddLocalRotation` (`self.SpringArm`) (`KismetMathLibrary.MakeRotator` 0.0 AxisValue) false false))

(event `InputAxis|Throttle`
  (params (AxisValue :type "Float (single-precision)"))
  ;[1 1 1] Movement
  (`TankMovementComponent.IntendMoveForward` (`self.TankMovement`) AxisValue))

(event `InputAction|Fire`
  (params (Key :type "Key Structure"))
  (bind _tankaiming (`self.TankAiming`))
  (bind _firingstatus (`TankAimingComponent.FiringStatus` _tankaiming))
  ;[1 1 1] Actions
  (:`Pressed`
    (`TankAimingComponent.Fire` _tankaiming)
    (if (`|EnumEquality` _firingstatus "Aiming")
      (`GameplayStatics.SpawnSoundAtLocation` "/Game/Sounds/TankShot_Cue.TankShot_Cue" (`SceneComponent.K2_GetComponentLocation` (`self.Tank`)) (struct) 1.0 1.0 0.0 (`self.ShotSoundAttenuation`) :!label _label)
      (elif (`|EnumEquality` _firingstatus "Locked")
        (goto _label)))))

(event `InputAxis|Turn`
  (params (AxisValue :type "Float (single-precision)"))
  ;[1 1 1] Movement
  (`TankMovementComponent.IntendTurnRight` (`self.TankMovement`) AxisValue))

(event `InputAction|SwapCam`
  (params (Key :type "Key Structure"))
  (:`Pressed`
    (`ActorComponent.ToggleActive` (`self.FirstPerson`))
    (`ActorComponent.ToggleActive` (`self.ThirdPerson`))))

(fn `Initialize HealthBarWidget`
  (bind _ashealth_bar (cast `/Game/UI/HealthBar` (`WidgetComponent.GetUserWidgetObject` (`self.Health`))))
  (set `/Game/UI/HealthBar.MyTank` self _ashealth_bar)
  (return))

(fn `UserConstructionScript`)